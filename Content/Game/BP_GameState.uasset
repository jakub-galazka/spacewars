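; BP_GameState tracks the level's enemy count and triggers the game-over menu on a win or loss.
; On BeginPlay it counts actors tagged "Enemy", and DecreaseEnemiesNumber lowers that count, calling WinGame at zero.
; WinGame sets IsPassed to true, while LoseGame skips that step; both add WB_GameOverMenu to the viewport.
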(event Custom|Win%20Game
  (Variables|Default|SetIsPassed? true)
  (bind _returnvalue (UserInterface|CreateWidget "/Game/UI/WB_GameOverMenu.WB_GameOverMenu_C"))
  (UserInterface|Viewport|AddtoViewport _returnvalue 0))

(event Custom|Lose%20Game
  (bind _returnvalue (UserInterface|CreateWidget "/Game/UI/WB_GameOverMenu.WB_GameOverMenu_C"))
  (UserInterface|Viewport|AddtoViewport _returnvalue 0))

(event Custom|Decrease%20Enemies%20Number
  (bind _result (Math|Integer|DecrementInt (Variables|Default|GetEnemiesNumer))
    (:%20%20
      (if (== _result 0)
        (CallFunction|WinGame)))))

(event EventBeginPlay
  (bind _outactors (Actor|GetAllActorswithTag "Enemy"))
  (Variables|Default|SetEnemiesNumer (Utilities|Array|Length _outactors)))

(event EventTick
  (params (DeltaSeconds :type Float%20%28single-precision%29)))

(fn ConstructionScript)