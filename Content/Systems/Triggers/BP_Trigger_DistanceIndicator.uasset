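; BP_Trigger_DistanceIndicator is a trigger that displays the player's distance to it on a WBP_DistanceIndicator widget component.
; While the indicator is visible, Tick converts the distance between player character and trigger to rounded meters and updates the widget text.
; The construction script applies the IsVisible flag to the widget component, and the inherited OnTrigger event hides it, which also stops the distance updates.
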(event EventBeginPlay
  (|CallParentFunction)
  (bind _aswbp_distance_indicator (Utilities|Casting|CastToWBP_DistanceIndicator (UserInterface|GetUserWidgetObject (Variables|Default|GetWidget))))
  (Variables|Default|SetDistanceIndicatorWidget _aswbp_distance_indicator))

(event Collision|EventActorBeginOverlap
  (params (OtherActor :type Actor%20Object%20Reference))
  (|CallParentFunction OtherActor) ; This node is disabled and will not be called.\nDrag off pins to build functionality.
)

(event EventTick
  (params (DeltaSeconds :type Float%20%28single-precision%29))
  (|CallParentFunction DeltaSeconds)
  (if (Variables|Default|GetIsVisible?)
    (CallFunction|UpdateDistanceIndicatorWidget)))

(event EventOnTrigger
  (|CallParentFunction)
  (CallFunction|ToggleDistanceIndicatorWidgetVisibility false))

(fn ConstructionScript
  (|CallParentFunction)
  (CallFunction|ToggleDistanceIndicatorWidgetVisibility (Variables|Default|GetIsVisible?)))

(fn UpdateDistanceIndicatorWidget
  (Default|SetDistanceDisplay (Variables|Default|GetDistanceIndicatorWidget) (Utilities|String|Append (Utilities|String|ToString(Integer) (Math|Float|Round (/ (Math|Vector|Distance(Vector) (Transformation|GetActorLocation (Game|GetPlayerCharacter 0)) (Transformation|GetActorLocation)) 1e+02))) " m")))

(fn ToggleDistanceIndicatorWidgetVisibility
  (params (IsVisible? :type Boolean))
  (bind _output_get (Variables|Default|SetIsVisible? IsVisible?))
  (Rendering|SetVisibility (Variables|Default|GetWidget) _output_get false))