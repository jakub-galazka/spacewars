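; BP_Trigger_Fence is a trigger-driven sci-fi fence that lowers out of the way when triggered.
; On the inherited OnTrigger event, it runs the parent logic, then checks CanTrigger before moving the fence mesh down to a fixed relative position over a short timed interpolation with MoveComponentTo.
; It has no reverse motion, and its other events and construction script add no logic.
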(event EventBeginPlay
  (|CallParentFunction) ; This node is disabled and will not be called.\nDrag off pins to build functionality.
)

(event Collision|EventActorBeginOverlap
  (params (OtherActor :type Actor%20Object%20Reference))
  (|CallParentFunction OtherActor) ; This node is disabled and will not be called.\nDrag off pins to build functionality.
)

(event EventTick
  (params (DeltaSeconds :type Float%20%28single-precision%29))
  (|CallParentFunction DeltaSeconds) ; This node is disabled and will not be called.\nDrag off pins to build functionality.
)

(event EventOnTrigger
  (|CallParentFunction)
  (if (Variables|Default|GetCanTrigger?)
    (Components|MoveComponentTo (Variables|Default|GetSM_Scifi_Fence_01) "0.000000,0.000000,-330.000000" "0, 0, 0" false false 1.5 false)))

(fn ConstructionScript
  (|CallParentFunction))