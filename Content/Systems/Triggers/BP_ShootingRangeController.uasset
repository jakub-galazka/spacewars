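; Shooting range controller that switches groups of range targets between covered and uncovered states.
; Cover and uncover events loop over a supplied target array, calling ToggleCover on each target and setting its IsOn flag off when covered, on when uncovered.
; A cover-all event runs the cover event on four stored round arrays.
; It has no active BeginPlay, Tick or overlap logic, and nothing within it triggers uncovering or cover-all.
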(event Custom|Cover%20Range%20Tragets
  (params (Range%20Targets :type Array%20of%20BP%20Range%20Target%20Object%20References))
  (for _array_element Range%20Targets
    (Default|ToggleCover _array_element true)
    (Variables|/Game/Systems/BP_RangeTarget.BP_RangeTarget_C|SetIsOn? _array_element false)))

(event Custom|Cover%20All%20Range%20Targets
  (CallFunction|CoverRangeTragets (Variables|Default|GetRound))
  (CallFunction|CoverRangeTragets (Variables|Default|GetRound_0))
  (CallFunction|CoverRangeTragets (Variables|Default|GetRound_1))
  (CallFunction|CoverRangeTragets (Variables|Default|GetRound_2)))

(event Custom|Uncover%20Range%20Targets
  (params (RangeTargets :type Array%20of%20BP%20Range%20Target%20Object%20References))
  (for _array_element RangeTargets
    (Default|ToggleCover _array_element false)
    (Variables|/Game/Systems/BP_RangeTarget.BP_RangeTarget_C|SetIsOn? _array_element true)))

(event EventBeginPlay)

(event Collision|EventActorBeginOverlap
  (params (OtherActor :type Actor%20Object%20Reference)))

(event EventTick
  (params (DeltaSeconds :type Float%20%28single-precision%29)))

(fn ConstructionScript)