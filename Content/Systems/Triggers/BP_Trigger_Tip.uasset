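; BP_Trigger_Tip is a trigger that shows a tip message on the player's HUD.
; It overrides OnTrigger, calls the parent implementation, then passes its Tip variable to ShowTipMessage on the first player controller's HUD with a fixed five-second duration.
; Trigger detection is left to the parent class, as the local BeginPlay, overlap and Tick events are disabled.
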(event EventBeginPlay
  (|CallParentFunction) ; This node is disabled and will not be called.\nDrag off pins to build functionality.
)

(event Collision|EventActorBeginOverlap
  (params (OtherActor :type Actor%20Object%20Reference))
  (|CallParentFunction OtherActor) ; This node is disabled and will not be called.\nDrag off pins to build functionality.
)

(event EventTick
  (params (DeltaSeconds :type Float%20%28single-precision%29))
  (|CallParentFunction DeltaSeconds) ; This node is disabled and will not be called.\nDrag off pins to build functionality.
)

(event EventOnTrigger
  (|CallParentFunction)
  (Class|BPIHUD|ShowTip(Message) (HUD|GetHUD (Game|GetPlayerController 0)) (Variables|Default|GetTip) 5.0))

(fn ConstructionScript
  (|CallParentFunction))