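; Tutorial-level easter egg trigger that spawns a wave of enemies when triggered.
; It overrides the parent trigger's OnTrigger, calls the parent, then spawns five BP_Enemy actors in an evenly spaced row at hard-coded world positions.
; It then recounts all actors tagged "Enemy" and writes the total to the enemy count on BP_GameState.
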(event EventBeginPlay
  (|CallParentFunction) ; This node is disabled and will not be called.\nDrag off pins to build functionality.
)

(event Collision|EventActorBeginOverlap
  (params (OtherActor :type Actor%20Object%20Reference))
  (|CallParentFunction OtherActor) ; This node is disabled and will not be called.\nDrag off pins to build functionality.
)

(event EventTick
  (params (DeltaSeconds :type Float%20%28single-precision%29))
  (|CallParentFunction DeltaSeconds) ; This node is disabled and will not be called.\nDrag off pins to build functionality.
)

(event EventOnTrigger
  (|CallParentFunction)
  (Game|SpawnActorfromClass "/Game/Characters/Enemy/BP_Enemy.BP_Enemy_C" (Math|Transform|MakeTransform "2030.000000,900.000000,116.000000" "0, 0, 0" "1.000000,1.000000,1.000000") "Undefined" "MultiplyWithRoot" 0 0)
  (Game|SpawnActorfromClass "/Game/Characters/Enemy/BP_Enemy.BP_Enemy_C" (Math|Transform|MakeTransform "2030.000000,1100.000000,116.000000" "0, 0, 0" "1.000000,1.000000,1.000000") "Undefined" "MultiplyWithRoot" 0 0)
  (Game|SpawnActorfromClass "/Game/Characters/Enemy/BP_Enemy.BP_Enemy_C" (Math|Transform|MakeTransform "2030.000000,1300.000000,116.000000" "0, 0, 0" "1.000000,1.000000,1.000000") "Undefined" "MultiplyWithRoot" 0 0)
  (Game|SpawnActorfromClass "/Game/Characters/Enemy/BP_Enemy.BP_Enemy_C" (Math|Transform|MakeTransform "2030.000000,1500.000000,116.000000" "0, 0, 0" "1.000000,1.000000,1.000000") "Undefined" "MultiplyWithRoot" 0 0)
  (Game|SpawnActorfromClass "/Game/Characters/Enemy/BP_Enemy.BP_Enemy_C" (Math|Transform|MakeTransform "2030.000000,1700.000000,116.000000" "0, 0, 0" "1.000000,1.000000,1.000000") "Undefined" "MultiplyWithRoot" 0 0)
  (bind _asbp_game_state (Utilities|Casting|CastToBP_GameState (Game|GetGameState)))
  (bind _outactors (Actor|GetAllActorswithTag "Enemy"))
  (Variables|/Game/Game/BP_GameState.BP_GameState_C|SetEnemiesNumer _asbp_game_state (Utilities|Array|Length _outactors)))

(fn ConstructionScript
  (|CallParentFunction))