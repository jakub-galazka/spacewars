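; Shooting range target that can slide side to side and flip in and out of cover until hit.
; BeginPlay starts two optional, randomly delayed loops that pause while IsOn is false: one alternates pitch, the other Y position, both through MoveComponentTo.
; Travel time scales with MoveRange.
; The first mesh hit plays a sound, sets IsHit to end both loops and rotates the target into cover.
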(event OnComponentHit(SM_RangeTarget)
  (params (HitComponent :type Primitive%20Component%20Object%20Reference) (OtherActor :type Actor%20Object%20Reference) (OtherComp :type Primitive%20Component%20Object%20Reference) (NormalImpulse :type Vector :default "0, 0, 0") (Hit :type Hit%20Result%20Structure%20%28by%20ref%29))
  (Utilities|FlowControl|DoOnce false
    (:Completed
      (Variables|Default|SetIsHit? true)
      (Audio|PlaySound2D "/Game/Audio/SoundWaves/SW_SwordHit.SW_SwordHit" 1.0 1.0 0.0 0 0)
      (CallFunction|ToggleCover true))))

(event Custom|Move%20Loop
  (bind _moverange (Variables|Default|GetMoveRange))
  ;[0.05098 0.05098 0.05098] Move Loop
  (if (Variables|Default|GetIsMoving?)
    (Utilities|FlowControl|Delay (Math|Random|RandomFloatinRange 0.5 1.5))
    (if (not (Variables|Default|GetIsHit?)) :!label _label
      (if (Variables|Default|GetIsOn?)
        (bind _isa (Utilities|FlowControl|FlipFlop)
          (:A
            _)
          (:B
            _))
        (Components|MoveComponentTo (Variables|Default|GetSM_RangeTarget) (Math|Vector|MakeVector 0.0 (Math|Float|SelectFloat _moverange (* _moverange -1.0) _isa) 0.0) "0, 0, 0" false false (/ (Math|Float|Absolute(Float) _moverange) 1e+03) false))
      (Utilities|FlowControl|Delay 0.5)
      (goto _label))))

(event Custom|Toggle%20Cover
  (params (ToggleCover? :type Boolean))
  (bind _moverange (Variables|Default|GetMoveRange))
  (bind _sm_rangetarget (Variables|Default|GetSM_RangeTarget))
  ;[0.05098 0.05098 0.05098] Cover
  (Components|MoveComponentTo _sm_rangetarget (Variables|/Script/Engine.SceneComponent|GetRelativeLocation _sm_rangetarget) (Math|Rotator|MakeRotator 0.0 (Math|Float|SelectFloat 9e+01 0.0 ToggleCover?) 0.0) true false 0.2 true)
  ;[0.05098 0.05098 0.05098] Move Loop
  (Components|MoveComponentTo (Variables|Default|GetSM_RangeTarget) (Math|Vector|MakeVector 0.0 (Math|Float|SelectFloat _moverange (* _moverange -1.0) (stale Custom|Move%20Loop _isa)) 0.0) "0, 0, 0" false false (/ (Math|Float|Absolute(Float) _moverange) 1e+03) false) ; enters at Stop
)

(event Custom|Cover%20Loop
  ;[0.05098 0.05098 0.05098] Cover Loop
  (if (Variables|Default|GetIsCovering?)
    (Utilities|FlowControl|Delay (Math|Random|RandomFloatinRange 1.0 3.0))
    (if (not (Variables|Default|GetIsHit?)) :!label _label
      (if (Variables|Default|GetIsOn?)
        (bind _isa (Utilities|FlowControl|FlipFlop)
          (:A
            _)
          (:B
            _))
        (CallFunction|ToggleCover _isa))
      (Utilities|FlowControl|Delay 1.5)
      (goto _label))))

(event EventBeginPlay
  (CallFunction|CoverLoop)
  (CallFunction|MoveLoop))

(event Collision|EventActorBeginOverlap
  (params (OtherActor :type Actor%20Object%20Reference)))

(event EventTick
  (params (DeltaSeconds :type Float%20%28single-precision%29)))

(fn ConstructionScript)