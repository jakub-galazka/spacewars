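; Rifle-armed enemy character that roams, hunts the player it sees, and ragdolls on death, decrementing the GameState enemy count.
; It loops moves to random reachable points until PawnSensing spots BP_Player, then moves within range and fires.
; Each shot faces the target, plays montage and sound, and spawns a projectile from the barrel with random spread.
; A retriggerable delay just longer than the sensing interval resumes roaming once sightings stop.
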(event OnSeePawn(PawnSensing)
  (params (Pawn :type Pawn%20Object%20Reference))
  ;[0.05098 0.05098 0.05098] Senses System
  (bind _asbp_player (Utilities|Casting|CastToBP_Player Pawn))
  (Variables|Default|SetIsSensing? true)
  (Utilities|FlowControl|Sequence
    (:then_0
      (CallFunction|ChaseTarget _asbp_player))
    (:then_1
      (Utilities|FlowControl|RetriggerableDelay (+ (Variables|/Script/AIModule.PawnSensingComponent|GetSensingInterval (Variables|Default|GetPawnSensing)) 0.1))
      (Variables|Default|SetIsSensing? false)
      (CallFunction|MoveAround))))

(event Custom|Move%20Around
  ;[0.05098 0.05098 0.05098] Move System
  (AI|AIMoveTo self (.RandomLocation (AI|Navigation|GetRandomReachablePointinRadius (Transformation|GetActorLocation) 2e+03 0 0)) 0 3e+02 false
    (:OnSuccess
      (Utilities|FlowControl|Delay 1.0)
      (CallFunction|MoveAround))))

(event Custom|Chase%20Target
  (params (TargetActor :type Actor%20Object%20Reference))
  ;[0.05098 0.05098 0.05098] Chase Target System
  (AI|AIMoveTo self "0, 0, 0" TargetActor 1e+03 false
    (:OnSuccess
      (CallFunction|Fire TargetActor))))

(event Custom|Fire
  (params (TargetActor :type Actor%20Object%20Reference))
  (bind _rifle (Variables|Default|GetRifle))
  (bind _returnvalue (Transformation|GetSocketTransform _rifle "Barrel" "RTS_World"))
  ;[0.05098 0.05098 0.05098] Fire System
  (bind _facerotation (CallFunction|FaceTarget TargetActor))
  ;;[1 1 1] TODO: Is it working?
  (Animation|PlayAnimMontage "/Game/Characters/Enemy/Animations/AM_Firing_Rifle.AM_Firing_Rifle" 1.0 "None")
  (Audio|PlaySoundatLocation "/Game/Audio/MetaSoundSources/MSS_BlasterShot.MSS_BlasterShot" (.location _returnvalue) "0, 0, 0" 1.0 1.0 0.0 0 0 0 0)
  (Game|SpawnActorfromClass "/Game/Projectiles/BP_Projectile_Enemy.BP_Projectile_Enemy_C" (Math|Transform|MakeTransform (.location _returnvalue) (Math|Rotator|CombineRotators _facerotation (Math|Rotator|MakeRotator (Math|Random|RandomFloatinRange -2.0 2.0) (Math|Random|RandomFloatinRange -2.0 2.0) (Math|Random|RandomFloatinRange -2.0 2.0))) "0.050000,0.050000,0.050000") "AlwaysSpawn" "MultiplyWithRoot" 0 0))

(event Game|Damage|EventAnyDamage
  (params (Damage :type Float%20%28single-precision%29) (DamageType :type Damage%20Type%20Object%20Reference) (InstigatedBy :type Controller%20Object%20Reference) (DamageCauser :type Actor%20Object%20Reference))
  ;[0.05098 0.05098 0.05098] Death System
  (bind _output_get (Variables|Default|SetHealth (- (Variables|Default|GetHealth) Damage)))
  (if (<= _output_get 0.0)
    (Utilities|FlowControl|DoOnce false
      (:Completed
        (Pawn|Components|CharacterMovement|DisableMovement (Variables|Character|GetCharacterMovement))
        (Class|PawnSensingComponent|SetSensingInterval (Variables|Default|GetPawnSensing) 0.0)
        (Physics|SetSimulatePhysics (Variables|Character|GetMesh) true)
        (bind _asbp_game_state (Utilities|Casting|CastToBP_GameState (Game|GetGameState)))
        (Default|DecreaseEnemiesNumber _asbp_game_state)))))

(event Collision|EventActorBeginOverlap
  (params (OtherActor :type Actor%20Object%20Reference)))

(event EventTick
  (params (DeltaSeconds :type Float%20%28single-precision%29)))

(event EventBeginPlay
  (CallFunction|MoveAround))

(fn ConstructionScript)

(fn FaceTarget
  (params (TargetActor :type Actor%20Object%20Reference))
  (bind _returnvalue (Transformation|GetActorLocation TargetActor))
  (bind _returnvalue_2 (Transformation|GetActorLocation))
  (bind _returnvalue_3 (Math|Rotator|FindLookatRotation _returnvalue_2 _returnvalue))
  (Transformation|SetActorRotation _returnvalue_3)
  (return _returnvalue_3))